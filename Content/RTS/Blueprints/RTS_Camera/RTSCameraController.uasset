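; Player controller for the RTS camera that pans the RTSCamera pawn with movement input.
; It caches the pawn on BeginPlay, then MoveForward and MoveRight offset its location along world X and Y while camera movement is enabled.
; Pan speed scales with spring arm length within clamped limits and doubles while Left Shift is held.
; Movement is applied per input tick without delta-time scaling.
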(event `self.ReceiveBeginPlay`
  (`|ExecutionSequence`
    (:`then_0`
      (bind _asrtscamera (cast `/Game/RTS/Blueprints/RTS_Camera/RTSCamera` (`GameplayStatics.GetPlayerPawn` 0)))
      (set `self.CameraRef` _asrtscamera))))

(event `InputAxis|MoveForward`
  (params (AxisValue :type "Float (single-precision)"))
  (if (and (`self.IsCameraMovementEnable`) (!= AxisValue 0.0))
    (`self.K2_SetActorLocation` (`self.CameraRef`) (+ (`KismetMathLibrary.MakeVector` (* AxisValue (`self.MoveSpeedMultiplier`) (`self.CalcMovementSpeed`))) (`self.K2_GetActorLocation` (`self.CameraRef`))) false false)))

(event `InputAxis|MoveRight`
  (params (AxisValue :type "Float (single-precision)"))
  (if (and (`self.IsCameraMovementEnable`) (!= AxisValue 0.0))
    (`self.K2_SetActorLocation` (`self.CameraRef`) (+ (`KismetMathLibrary.MakeVector` 0.0 (* AxisValue (`self.MoveSpeedMultiplier`) (`self.CalcMovementSpeed`))) (`self.K2_GetActorLocation` (`self.CameraRef`))) false false)))

(event `Key|LeftShift`
  (params (Key :type "Key Structure"))
  (:`Pressed`
    (set `self.MoveSpeedMultiplier` 2.0))
  (:`Released`
    (set `self.MoveSpeedMultiplier` 1.0)))

(fn `CalcMovementSpeed`
  (returns (ReturnValue :type "Float (double-precision)"))
  (return (`KismetMathLibrary.FClamp` (/ (`SpringArmComponent.TargetArmLength` (`/Game/RTS/Blueprints/RTS_Camera/RTSCamera.SpringArm` (`self.CameraRef`))) 100.0) 5.0 20.0)))

(fn `UserConstructionScript`)